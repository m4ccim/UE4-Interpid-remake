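; A replicated bomb projectile that arms when it bounces and explodes after a fuse delay.
; The authority sets Armed and starts the fuse timer on bounce, and the Armed RepNotify turns the mesh red through a dynamic material instance.
; On expiry, the authority damages pawns within the explosion radius, triggers OnExplosion to spawn effects and hide the bomb, then sets a short lifespan for cleanup.
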(event OnProjectileBounce(ProjectileMovement)
  (params (ImpactResult :type Hit%20Result%20Structure%20%28by%20ref%29) (ImpactVelocity :type Vector%20%28by%20ref%29 :default "0, 0, 0"))
  (Networking|SwitchHasAuthority
    (:Authority
      (Variables|Default|SetArmed true)
      (Utilities|Time|SetTimerbyFunctionName 0 "OnBombFuseExpired" (Variables|Default|GetFuseTime)))))

(event Custom|OnExplosion
  (Effects|SpawnEmitteratLocation (Variables|Default|GetExplosionEffects) (Transformation|GetActorLocation))
  (Collision|SetActorEnableCollision false)
  (Rendering|SetActorHiddenInGame true))

(event EventBeginPlay)

(event Collision|EventActorBeginOverlap
  (params (OtherActor :type Actor%20Object%20Reference)))

(event EventTick
  (params (DeltaSeconds :type Float%20%28single-precision%29)))

(fn ConstructionScript
  (bind _returnvalue (Rendering|Material|CreateDynamicMaterialInstance (Variables|Default|GetBombMesh) 0 0 "None" :!class /Script/Engine.PrimitiveComponent))
  (Variables|Default|SetBombMID _returnvalue)
  (CallFunction|SetBombColor))

(fn OnRepArmed
  (if (Variables|Default|GetArmed)
    (CallFunction|SetBombColor "(R=1.000000,G=0.000000,B=0.007126,A=1.000000)")))

(fn SetBombColor
  (params (BombColor :type Linear%20Color%20Structure))
  (Rendering|Material|SetVectorParameterValue (Variables|Default|GetBombMID) (Variables|Default|GetMaterialColorParam) BombColor :!class /Script/Engine.MaterialInstanceDynamic))

(fn OnBombFuseExpired
  (Networking|SwitchHasAuthority
    (:Authority
      (CallFunction|ApplyExplosionDamage)
      (CallFunction|OnExplosion)
      (Actor|SetLifeSpan 2.0))))

(fn ApplyExplosionDamage
  (bind _outactors (Collision|SphereOverlapActors (Transformation|GetActorLocation) (Variables|Default|GetExplosionRadius) (Utilities|Array|MakeArray "ObjectTypeQuery3") 0))
  (for _array_element _outactors
    (Game|Damage|ApplyDamage _array_element (Variables|Default|GetExplosionDamage) (Game|GetInstigatorController) self "/Script/Engine.DamageType")))