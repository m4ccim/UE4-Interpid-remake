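; Heal_BP is a healing pickup actor that spins in place.
; When a ThirdPersonCharacter overlaps it, it calls that character's AttemptPickupHeal with itself, leaving the pickup logic to the character.
; Tick applies a frame-rate-independent yaw rotation, and BeginPlay caches a reference to the player character, which the graph does not otherwise use.
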(event EventBeginPlay
  (bind _asthird_person_character (Utilities|Casting|CastToThirdPersonCharacter (Game|GetPlayerCharacter 0)))
  (Variables|Default|SetPlayerCharacter _asthird_person_character))

(event Collision|EventActorBeginOverlap
  (params (OtherActor :type Actor%20Object%20Reference))
  (bind _asthird_person_character (Utilities|Casting|CastToThirdPersonCharacter OtherActor))
  (Default|AttemptPickupHeal _asthird_person_character self))

(event EventTick
  (params (DeltaSeconds :type Float%20%28single-precision%29))
  (Transformation|AddActorLocalRotation (* (Math|Rotator|MakeRotator 0.0 0.0 1e+02) DeltaSeconds) false false))

(fn ConstructionScript)